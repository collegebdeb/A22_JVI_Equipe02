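; Patrol route for enemies that holds a list of patrol points and tracks the current index.
; On BeginPlay it starts at the configured first index and, for non-looping routes, appends the interior points in reverse to create a back-and-forth cycle.
; IncrementPatrolPointIndex advances with modulo wrap-around and returns the new index, so both route types share the same stepping logic.
; An empty route prints an on-screen warning at BeginPlay.
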(event `self.ReceiveBeginPlay`
  (bind _patrolpointlist (`self.PatrolPointList`))
  (if (!= (`KismetArrayLibrary.Array_Length` (`self.PatrolPointList`)) 0)
    (set `self.CurrentPatrolPointIndex` (`self.FirstPatrolPointIndex`))
    (if (not (`self.IsLooping`))
      ;[1 1 1] Adds the reversed list to the list if the route is not looping
      (bind (_arrayindex _arrayelement) (`/Engine/EditorBlueprintResources/StandardMacros.ReverseForEachLoop` _patrolpointlist)
        (:`LoopBody`
          (if (`KismetMathLibrary.BooleanNOR` (== _arrayindex 0) (== _arrayindex (- (`KismetArrayLibrary.Array_Length` _patrolpointlist) 1)))
            (`KismetArrayLibrary.Array_Add` _patrolpointlist _arrayelement)))))
    (else
      ;[1 1 1] Warning if the route is empty
      (`KismetSystemLibrary.PrintString` (`KismetStringLibrary.Concat_StrStr` (`KismetSystemLibrary.GetDisplayName` self) " is empty") true true (struct :`R` 1.0 :`B` 0.042226 :`A` 1.0) 5.0))))

(fn `IncrementPatrolPointIndex`
  (returns (CurrentPatrolPointIndex :type Integer))
  (bind _output_get (set `self.CurrentPatrolPointIndex` (mod (+ (`self.CurrentPatrolPointIndex`) 1) (`KismetArrayLibrary.Array_Length` (`self.PatrolPointList`)))))
  (return _output_get))

(fn `UserConstructionScript`)