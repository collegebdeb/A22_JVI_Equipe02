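; Parent Blueprint for cosmetic billboards with animated emissive materials and an optional point light, configured entirely in the Construction Script.
; It takes the primitive at child index 2 of BillboardRoot and feeds texture, color, opacity, flash, wave and glitch settings into a dynamic material instance.
; A random time offset varies effect timing per construction.
; When enabled, the movable light can auto-fit its position, source length and rotation to the mesh bounds.
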(fn `UserConstructionScript`
  (locals (billboard :type "PrimitiveComponent Object Reference") (Local_lightLocation :type "Vector Structure") (Local_billboardHeight :type "Float (double-precision)"))
  (bind _pointlight (`self.PointLight`))
  (bind _pointlight_2 (`self.PointLight`))
  (bind (_returnvalue_location _returnvalue_rotation _returnvalue_scale) (`KismetMathLibrary.BreakTransform` (`SceneComponent.GetRelativeTransform` (`self.PointLight`))))
  (bind (_origin _boxextent) (`KismetSystemLibrary.GetComponentBounds` (`local.billboard`)))
  (bind (_origin_2 _boxextent_2) (`KismetSystemLibrary.GetComponentBounds` (`local.billboard`)))
  (bind _returnvalue (`SceneComponent.GetChildComponent` (`self.BillboardRoot`) 2))
  (bind (_relativerotation_roll _relativerotation_pitch _relativerotation_yaw) (`KismetMathLibrary.BreakRotator` (`SceneComponent.RelativeRotation` _pointlight_2)))
  (bind _returnvalue_2 (`KismetMathLibrary.GetMaxElement` _boxextent))
  (`/Engine/EditorBlueprintResources/StandardMacros.IsValid` _returnvalue
    (:`Is Valid`
      (bind _asprimitive_component (cast `PrimitiveComponent` _returnvalue))
      (set `local.billboard` _asprimitive_component)
      (`|ExecutionSequence`
        (:`then_0`
          (bind _returnvalue_3 (`PrimitiveComponent.CreateDynamicMaterialInstance` (`local.billboard`) 0 (`self.MasterMaterial`) "None"))
          (bind _output_get (set `self.DynamicMaterialInstance` _returnvalue_3))
          (`MaterialInstanceDynamic.SetScalarParameterValue` _output_get "Opacity" (`self.Opacity`))
          (`PrimitiveComponent.SetMaterial` (`local.billboard`) 0 (`self.DynamicMaterialInstance`))
          (`MaterialInstanceDynamic.SetTextureParameterValue` (`self.DynamicMaterialInstance`) "Billboard_Texture" (`self.BillboardTexture`))
          (`MaterialInstanceDynamic.SetVectorParameterValue` (`self.DynamicMaterialInstance`) "Emissive_Color" (`self.EmissiveColor`))
          ;[1 1 1] Flash
          (`MaterialInstanceDynamic.SetScalarParameterValue` (`self.DynamicMaterialInstance`) "bFlash" (`KismetMathLibrary.Conv_BoolToDouble` (`self.bFlash?`)))
          (`MaterialInstanceDynamic.SetScalarParameterValue` (`self.DynamicMaterialInstance`) "Flash_Period" (`self.FlashPeriod`))
          (`MaterialInstanceDynamic.SetScalarParameterValue` (`self.DynamicMaterialInstance`) "Flash_Minimum" (`self.FlashMinimum`))
          (`MaterialInstanceDynamic.SetScalarParameterValue` (`self.DynamicMaterialInstance`) "Flash_Power" (`self.FlashPower`))
          ;[1 1 1] Wave
          (`MaterialInstanceDynamic.SetTextureParameterValue` (`self.DynamicMaterialInstance`) "Wave_Texture" (`self.WaveTexture`))
          (`MaterialInstanceDynamic.SetScalarParameterValue` (`self.DynamicMaterialInstance`) "bWave" (`KismetMathLibrary.Conv_BoolToDouble` (`self.bWave?`)))
          (`MaterialInstanceDynamic.SetVectorParameterValue` (`self.DynamicMaterialInstance`) "Wave_Speed" (`KismetMathLibrary.MakeColor` (`self.WaveSpeedX`) (`self.WaveSpeedY`)))
          (`MaterialInstanceDynamic.SetScalarParameterValue` (`self.DynamicMaterialInstance`) "Wave_Intensity" (`self.WaveIntensity`))
          (`MaterialInstanceDynamic.SetScalarParameterValue` (`self.DynamicMaterialInstance`) "Wave_Contrast" (`self.WaveContrast`))
          (`MaterialInstanceDynamic.SetScalarParameterValue` (`self.DynamicMaterialInstance`) "bIsVertical" (`KismetMathLibrary.Conv_BoolToDouble` (`self.IsVertical`)))
          ;[1 1 1] Glitch
          (`MaterialInstanceDynamic.SetScalarParameterValue` (`self.DynamicMaterialInstance`) "Time_Offset" (`KismetMathLibrary.RandomFloatInRange` 0.0 10.0))
          (`MaterialInstanceDynamic.SetScalarParameterValue` (`self.DynamicMaterialInstance`) "bGlitch" (`KismetMathLibrary.Conv_BoolToDouble` (`self.bGlitch`)))
          (`MaterialInstanceDynamic.SetScalarParameterValue` (`self.DynamicMaterialInstance`) "Glitch1_Intensity" (`self.Glitch1_Intensity`))
          (`MaterialInstanceDynamic.SetScalarParameterValue` (`self.DynamicMaterialInstance`) "Glitch2_Intensity" (`self.Glitch2_Intensity`))
          (`MaterialInstanceDynamic.SetScalarParameterValue` (`self.DynamicMaterialInstance`) "Glitch_Repeat" (`self.GlitchRepeat`))
          (`MaterialInstanceDynamic.SetScalarParameterValue` (`self.DynamicMaterialInstance`) "Glitch1_Delay" (`self.Glitch1_Delay`))
          (`MaterialInstanceDynamic.SetScalarParameterValue` (`self.DynamicMaterialInstance`) "Glitch2_Delay" (`self.Glitch2_Delay`))
          (`MaterialInstanceDynamic.SetScalarParameterValue` (`self.DynamicMaterialInstance`) "Glitch1_Flash_Duration" (`self.Glitch1_Flash_Duration`))
          (`MaterialInstanceDynamic.SetScalarParameterValue` (`self.DynamicMaterialInstance`) "Glitch2_Flash_Duration" (`self.Glitch2_Flash_Duration`)))
        (:`then_1`
          (if (`self.bAddLight`)
            (`SceneComponent.SetMobility` _pointlight "Movable")
            (`SceneComponent.SetHiddenInGame` _pointlight false true)
            (`SceneComponent.SetVisibility` _pointlight true true)
            (if (`self.bAutoSetLightLengthAndLocation`)
              (set `local.Local_lightLocation` _origin_2)
              (set `local.Local_billboardHeight` (* 2 (`KismetMathLibrary.GetMaxElement` _boxextent_2)))
              (`SceneComponent.K2_SetRelativeTransform` (`self.PointLight`) (`KismetMathLibrary.MakeTransform` (+ (`KismetMathLibrary.InverseTransformLocation` (`SceneComponent.K2_GetComponentToWorld` (`self.BillboardRoot`)) (`local.Local_lightLocation`)) _returnvalue_location) _returnvalue_rotation _returnvalue_scale) false false)
              (`PointLightComponent.SetSourceLength` (`self.PointLight`) (`local.Local_billboardHeight`))
              (`|ExecutionSequence`
                (:`then_0`
                  (if (== _returnvalue_2 (.y _boxextent))
                    (`SceneComponent.K2_SetRelativeRotation` _pointlight_2 (`KismetMathLibrary.MakeRotator` 90.0 _relativerotation_pitch _relativerotation_yaw) false false)))
                (:`then_1`
                  (if (== _returnvalue_2 (.z _boxextent))
                    (`SceneComponent.K2_SetRelativeRotation` _pointlight_2 (`KismetMathLibrary.MakeRotator` _relativerotation_roll _relativerotation_pitch 90.0) false false)))))
            (else
              (`SceneComponent.SetMobility` _pointlight "Movable")
              (`SceneComponent.SetHiddenInGame` _pointlight true true)
              (`SceneComponent.SetVisibility` _pointlight false true))))))))