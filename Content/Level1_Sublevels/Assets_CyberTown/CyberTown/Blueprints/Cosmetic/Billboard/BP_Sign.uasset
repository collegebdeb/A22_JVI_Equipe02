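; BP_Sign is a cosmetic CyberTown sign that displays one selectable image from a shared texture atlas, noted as a 6x6 grid.
; The construction script clamps SignSelection to the grid's cell count, derived from TextureSliceSize.
; It converts the index into column and row UV offsets and writes them to scalar parameters on DynamicMaterialInstance.
; The event graph has only disabled default events.
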(fn `UserConstructionScript`
  (bind _textureslicesize (`self.TextureSliceSize`))
  (bind _returnvalue (`KismetMathLibrary.Conv_IntToDouble` (`self.SignSelection`)))
  (bind _returnvalue_2 (`KismetMathLibrary.Conv_IntToDouble` (`self.TextureSliceSize`)))
  (`parent.UserConstructionScript`)
  ;[1 1 1] Texture Slicing [The sign textures are all in a 6x6 texture] -> We need to offset the UV in a way to show one at a time
  ;;[0 0.1553 1] Clamp sign selection the number of available sign textures
  (set `self.SignSelection` (`KismetMathLibrary.Clamp` (`self.SignSelection`) 0 (- (* _textureslicesize _textureslicesize) 1)))
  (`MaterialInstanceDynamic.SetScalarParameterValue` (`self.DynamicMaterialInstance`) "Horizontal_Offset_Num" (/ (mod _returnvalue _returnvalue_2) _returnvalue_2))
  (`MaterialInstanceDynamic.SetScalarParameterValue` (`self.DynamicMaterialInstance`) "Vertical_Offset_Num" (/ (`KismetMathLibrary.Conv_IntToDouble` (`.ReturnValue` (`KismetMathLibrary.FMod` _returnvalue _returnvalue_2))) (`KismetMathLibrary.Conv_IntToDouble` (`self.TextureSliceSize`)))))