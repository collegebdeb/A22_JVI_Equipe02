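; Moving platform Blueprint, named as a sinking platform, that travels toward an end position while the player overlaps its trigger and returns when they leave.
; The MovePlatforme timeline lerps the mesh's relative location from its starting point to EndLocation, playing or reversing at a rate set by a duration variable.
; The construction script applies mesh, scale and rotation to both the platform and a reference mesh marking the end position.
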(event `self.ReceiveBeginPlay`
  (set `self.Start location` (`SceneComponent.RelativeLocation` (`self.mainPlatform`))))

(event `self.collisionBiscuit.OnComponentBeginOverlap`
  (params (OverlappedComponent :type "PrimitiveComponent Object Reference") (OtherActor :type "Actor Object Reference") (OtherComp :type "PrimitiveComponent Object Reference") (OtherBodyIndex :type Integer) (bFromSweep :type Boolean) (SweepResult :type "HitResult Structure (by ref)"))
  (cast `/Game/HackerZ/Blueprints/Player/BP_Player` OtherActor)
  (`TimelineComponent.SetPlayRate` (`self.Move platforme`) (/ 1.0 (`self.duration(seconde)`)))
  (bind (_direction _move_track) (`Timeline|Move platforme` :!label _label)
    (:`Update`
      (`SceneComponent.K2_SetRelativeLocation` (`self.mainPlatform`) (`KismetMathLibrary.VLerp` (`self.Start location`) (`self.End Location`) _move_track) false false))))

(event `self.collisionBiscuit.OnComponentEndOverlap`
  (params (OverlappedComponent :type "PrimitiveComponent Object Reference") (OtherActor :type "Actor Object Reference") (OtherComp :type "PrimitiveComponent Object Reference") (OtherBodyIndex :type Integer))
  (cast `/Game/HackerZ/Blueprints/Player/BP_Player` OtherActor)
  (`TimelineComponent.SetPlayRate` (`self.Move platforme`) (/ 1.0 (`self.duration(seconde)`)))
  (goto _label :!via `Reverse`))

(fn `UserConstructionScript`
  (bind _mainplatform (`self.mainPlatform`))
  (bind _end_platform_reference (`self.End Platform reference`))
  (bind _platforme_mesh (`self.Platforme mesh`))
  (`StaticMeshComponent.SetStaticMesh` _mainplatform _platforme_mesh)
  (`StaticMeshComponent.SetStaticMesh` _end_platform_reference _platforme_mesh)
  (`SceneComponent.SetRelativeScale3D` _mainplatform (`self.Scale`))
  (`SceneComponent.SetRelativeScale3D` _end_platform_reference (`self.Scale`))
  (`SceneComponent.K2_SetRelativeRotation` _mainplatform (`self. Rotation`) false false)
  (`SceneComponent.K2_SetRelativeRotation` _end_platform_reference (`self. Rotation`) false false)
  (`SceneComponent.K2_SetRelativeLocation` _end_platform_reference (`self.End Location`) false false))