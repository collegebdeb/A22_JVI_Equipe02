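; Disappearing biscuit platform that vanishes shortly after the player steps on it, then reappears.
; When BP_Player begins overlapping Collision_biscuit, BiscuitChoco gets BaseMaterial, then after a short delay loses collision and is hidden.
; When any overlap with that trigger ends, a matching delay restores the mesh's material, visibility and collision, with no player check.
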(event `self.collision_biscuit.OnComponentBeginOverlap`
  (params (OverlappedComponent :type "PrimitiveComponent Object Reference") (OtherActor :type "Actor Object Reference") (OtherComp :type "PrimitiveComponent Object Reference") (OtherBodyIndex :type Integer) (bFromSweep :type Boolean) (SweepResult :type "HitResult Structure (by ref)"))
  (cast `/Game/HackerZ/Blueprints/Player/BP_Player` OtherActor)
  (`PrimitiveComponent.SetMaterial` (`self.Biscuit_Choco`) 0 "/Game/FPWeapon/Materials/BaseMaterial.BaseMaterial")
  (`KismetSystemLibrary.Delay` 1.0)
  (`PrimitiveComponent.SetCollisionEnabled` (`self.Biscuit_Choco`) "NoCollision")
  (`SceneComponent.SetVisibility` (`self.Biscuit_Choco`) false false))

(event `self.collision_biscuit.OnComponentEndOverlap`
  (params (OverlappedComponent :type "PrimitiveComponent Object Reference") (OtherActor :type "Actor Object Reference") (OtherComp :type "PrimitiveComponent Object Reference") (OtherBodyIndex :type Integer))
  (`KismetSystemLibrary.Delay` 1.0)
  (`PrimitiveComponent.SetMaterial` (`self.Biscuit_Choco`) 0 "/Game/FPWeapon/Materials/BaseMaterial.BaseMaterial")
  (`SceneComponent.SetVisibility` (`self.Biscuit_Choco`) true false)
  (`PrimitiveComponent.SetCollisionEnabled` (`self.Biscuit_Choco`) "QueryAndPhysics"))

(fn `UserConstructionScript`)