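; Player component that acts as a pocket hacking tool, adding the HUD widget and managing a regenerating pool of hacking points.
; Each tick it traces from the camera, shows hacking GUI on BPI_Hacked targets and updates the FirstPersonHUD hackable flag.
; The player's hack event triggers a trace that calls the target's interface, drawing a beam effect from the right hand on success.
; Helper functions check and spend points.
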(event `self.ReceiveBeginPlay`
  (bind _asbp_player (cast `/Game/HackerZ/Blueprints/Player/BP_Player` (`self.GetOwner`)))
  (add `/Game/HackerZ/Blueprints/Player/BP_Player.OnHackEventDispatcher` _asbp_player (delegate `Hack`))
  ;[1 1 1] Ajoute le UI de hacking au HUD du joueur
  (bind _returnvalue (`|CreateWidget` "/Game/HackerZ/HUD/W_HUD.W_HUD_C" (`GameplayStatics.GetPlayerController` 0)))
  (`UserWidget.AddToViewport` _returnvalue 0))

(event `Hack`
  (bind _returnvalue (`GameplayStatics.GetPlayerCameraManager` 0))
  (bind _returnvalue_2 (`PlayerCameraManager.GetCameraLocation` _returnvalue))
  (bind (_outhit _returnvalue_3) (`KismetSystemLibrary.LineTraceSingle` :`Start` _returnvalue_2 :`End` (+ _returnvalue_2 (* (`Actor.GetActorForwardVector` _returnvalue) (`self.HackDistance`))) :`TraceChannel` "TraceTypeQuery1" :`DrawTime` 0.3))
  (if _returnvalue_3
    (bind (_bblockinghit _binitialoverlap _time _distance _location _impactpoint _normal _impactnormal _physmat _hitactor) (`GameplayStatics.BreakHitResult` _outhit))
    (cast `/Game/HackerZ/Blueprints/InteractableObjects/Blueprints/BPI_Hacked` _hitactor)
    (bind (_hacked _ishacked) (message `/Game/HackerZ/Blueprints/InteractableObjects/Blueprints/BPI_Hacked.GetHacked` _hitactor (`self.HackTime`) self))
    (if _ishacked
      (`self.DrawBeamFX` _location))))

(event `self.ReceiveTick`
  (params (DeltaSeconds :type "Float (single-precision)"))
  (bind _returnvalue (`GameplayStatics.GetPlayerCameraManager` 0))
  (bind _returnvalue_2 (`PlayerController.GetHUD` (`GameplayStatics.GetPlayerController` 0)))
  (bind _returnvalue_3 (`PlayerCameraManager.GetCameraLocation` _returnvalue))
  (set `self.HackingPoints` (`KismetMathLibrary.FClamp` (+ (* DeltaSeconds (`self.HackingPointsRecoveryMultiplier`)) (`self.HackingPoints`)) 0.0 (`self.MaxHackingPoints`)))
  (`|ExecutionSequence`
    (:`then_0`
      (bind (_outhit _returnvalue_4) (`KismetSystemLibrary.LineTraceSingle` :`Start` _returnvalue_3 :`End` (+ _returnvalue_3 (* (`Actor.GetActorForwardVector` _returnvalue) (`self.HackDistance`))) :`TraceChannel` "TraceTypeQuery1" :`TraceColor` (struct :`R` 0.137538 :`G` 1.0 :`B` 0.009595 :`A` 1.0) :`TraceHitColor` (struct :`G` 0.722498 :`B` 1.0 :`A` 1.0)))
      (if _returnvalue_4
        (bind _asbpi_hacked (cast `/Game/HackerZ/Blueprints/InteractableObjects/Blueprints/BPI_Hacked` (`.HitActor` (`GameplayStatics.BreakHitResult` _outhit)))
          (:`then`
            (`/Game/HackerZ/Blueprints/InteractableObjects/Blueprints/BPI_Hacked.DisplayHackingGUI` _asbpi_hacked self)
            (bind _asfirst_person_hud (cast `/Game/HackerZ/Blueprints/Player/FirstPersonBP/Blueprints/FirstPersonHUD` _returnvalue_2))
            (set `/Game/HackerZ/Blueprints/Player/FirstPersonBP/Blueprints/FirstPersonHUD.IsTargetHackable` true _asfirst_person_hud))
          (:`CastFailed`
            (bind _asfirst_person_hud_2 (cast `/Game/HackerZ/Blueprints/Player/FirstPersonBP/Blueprints/FirstPersonHUD` _returnvalue_2))
            (set `/Game/HackerZ/Blueprints/Player/FirstPersonBP/Blueprints/FirstPersonHUD.IsTargetHackable` false _asfirst_person_hud_2)))))))

(fn `DrawBeamFX`
  (params (EndBeamLocation :type "Vector Structure"))
  (bind _asbp_player (cast `/Game/HackerZ/Blueprints/Player/BP_Player` (`self.GetOwner`)))
  (bind _returnvalue (`NiagaraFunctionLibrary.SpawnSystemAtLocation` "/Game/HackerZ/FX/FXS_HackingBeam.FXS_HackingBeam" (`self.GetSocketLocation` (`/Game/HackerZ/Blueprints/Player/BP_Player.FirstPersonMesh_Arms` _asbp_player) "hand_r")))
  (`FXSystemComponent.SetVectorParameter` _returnvalue "User.BeamEnd" EndBeamLocation))

(fn `HasEnoughHackingPoints`
  (params (HackingPointsRequired :type "Float (double-precision)"))
  (returns (`Enough?` :type Boolean))
  (return (<= HackingPointsRequired (`self.HackingPoints`))))

(fn `SpendHackingPoints`
  (params (HackingPointsToSpend :type "Float (double-precision)"))
  (returns (IsEnoughPoints :type Boolean))
  (if (>= (`self.HackingPoints`) HackingPointsToSpend)
    (set `self.HackingPoints` (`KismetMathLibrary.FClamp` (- (`self.HackingPoints`) (`local.HackingPointsToSpend`)) 0.0 100.0))
    (return true)
    (else
      (return false))))