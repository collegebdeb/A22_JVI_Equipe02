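; BP_TriggerSaveGame is a save point trigger that saves the game when the player overlaps it.
; On overlap by a BP_Player, it calls OnSave on FirstPersonGameMode with the Capsule's world location and rotation plus the player's health.
; The saved transform therefore comes from the trigger's capsule rather than the player.
; The construction script divides the Capsule's relative scale and location by the Scene's world scale to offset actor scaling.
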(event `self.ReceiveActorBeginOverlap`
  (params (OtherActor :type "Actor Object Reference"))
  (bind _capsule (`self.Capsule`))
  (bind _asbp_player (cast `/Game/HackerZ/Blueprints/Player/BP_Player` OtherActor))
  (bind _asfirst_person_game_mode (cast `/Game/HackerZ/Blueprints/Game/FirstPersonGameMode` (`GameplayStatics.GetGameMode`)))
  (`/Game/HackerZ/Blueprints/Game/FirstPersonGameMode.OnSave` _asfirst_person_game_mode (`SceneComponent.K2_GetComponentLocation` _capsule) (`/Game/HackerZ/Blueprints/Player/BP_Player.Player Health` _asbp_player) (`SceneComponent.K2_GetComponentRotation` _capsule)))

(fn `UserConstructionScript`
  (bind _capsule (`self.Capsule`))
  (bind _capsule_2 (`self.Capsule`))
  (`SceneComponent.SetRelativeScale3D` _capsule (/ (`SceneComponent.RelativeScale3D` _capsule) (`SceneComponent.K2_GetComponentScale` (`self.Scene`))))
  (`SceneComponent.K2_SetRelativeLocation` _capsule_2 (/ (`SceneComponent.RelativeLocation` _capsule_2) (`SceneComponent.K2_GetComponentScale` (`self.Scene`))) false false))