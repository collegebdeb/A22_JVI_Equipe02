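; BP_Wallrun_Block is a volume that blocks wallrunning for a BP_Player that overlaps it.
; On actor overlap it finds the player's BPAC_WallRun component and clears CanWallrun.
; When the player leaves the Box component it sets CanWallrun back to true only if WallrunMode is Every Surface.
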(event `self.ReceiveActorBeginOverlap`
  (params (OtherActor :type "Actor Object Reference"))
  (bind _asbp_player (cast `/Game/HackerZ/Blueprints/Player/BP_Player` OtherActor))
  (bind _returnvalue (`self.GetComponentByClass` _asbp_player "/Game/HackerZ/Blueprints/Player/Components/BPAC_WallRun.BPAC_WallRun_C"))
  (`/Engine/EditorBlueprintResources/StandardMacros.IsValid` _returnvalue
    (:`Is Valid`
      (set `/Game/HackerZ/Blueprints/Player/Components/BPAC_WallRun.CanWallrun` false _returnvalue))))

(event `self.Box.OnComponentEndOverlap`
  (params (OverlappedComponent :type "PrimitiveComponent Object Reference") (OtherActor :type "Actor Object Reference") (OtherComp :type "PrimitiveComponent Object Reference") (OtherBodyIndex :type Integer))
  (bind _asbp_player (cast `/Game/HackerZ/Blueprints/Player/BP_Player` OtherActor))
  (bind _returnvalue (`self.GetComponentByClass` _asbp_player "/Game/HackerZ/Blueprints/Player/Components/BPAC_WallRun.BPAC_WallRun_C"))
  (`/Engine/EditorBlueprintResources/StandardMacros.IsValid` _returnvalue
    (:`Is Valid`
      (switch `/Game/HackerZ/Blueprints/Player/Components/WallrunModeEnum` (`/Game/HackerZ/Blueprints/Player/Components/BPAC_WallRun.WallrunMode` _returnvalue)
        (:`NewEnumerator0`
          (set `/Game/HackerZ/Blueprints/Player/Components/BPAC_WallRun.CanWallrun` true _returnvalue))))))

(fn `UserConstructionScript`)