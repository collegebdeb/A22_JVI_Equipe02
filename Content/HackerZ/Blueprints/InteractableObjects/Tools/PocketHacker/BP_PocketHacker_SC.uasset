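; Pocket hacker component for the player that lets them hack objects in view at range, using a regenerating pool of hacking points.
; It binds to the owning BP_Player's hack dispatcher, line traces from the camera and sends GetHackedMessage to the hit actor with the hack time and itself.
; SpendHackingPoints deducts points and reports success, while Tick refills them and prints the total on screen.
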(event `self.ReceiveBeginPlay`
  (bind _asbp_player (cast `/Game/HackerZ/Blueprints/Player/BP_Player` (`self.GetOwner`)))
  (add `/Game/HackerZ/Blueprints/Player/BP_Player.OnHackEventDispatcher` _asbp_player (delegate `Hack`)))

(event `Hack`
  (bind _returnvalue (`GameplayStatics.GetPlayerCameraManager` 0))
  (bind _returnvalue_2 (`PlayerCameraManager.GetCameraLocation` _returnvalue))
  (bind (_outhit _returnvalue_3) (`KismetSystemLibrary.LineTraceSingle` :`Start` _returnvalue_2 :`End` (+ _returnvalue_2 (* (`Actor.GetActorForwardVector` _returnvalue) (`self.HackDistance`))) :`TraceChannel` "TraceTypeQuery1" :`DrawDebugType` "ForDuration" :`DrawTime` 0.3))
  (if _returnvalue_3
    (message `/Game/HackerZ/Blueprints/InteractableObjects/Blueprints/BPI_Hacked.GetHacked` (`.HitActor` (`GameplayStatics.BreakHitResult` _outhit)) (`self.HackTime`) self)))

(event `self.ReceiveTick`
  (params (DeltaSeconds :type "Float (single-precision)"))
  (set `self.HackingPoints` (`KismetMathLibrary.FClamp` (+ (* DeltaSeconds (`self.HackingPointsRecoveryMultiplier`)) (`self.HackingPoints`)) 0.0 100.0))
  (`KismetSystemLibrary.PrintString` (`KismetStringLibrary.Concat_StrStr` "Pocket Hacker Points : " (`KismetStringLibrary.Conv_IntToString` (`KismetMathLibrary.Round` (`self.HackingPoints`)))) true false (struct :`R` 0.075322 :`G` 1.0 :`A` 1.0) 0.0))

(fn `SpendHackingPoints`
  (params (HackingPointsToSpend :type "Float (double-precision)"))
  (returns (IsEnoughPoints :type Boolean))
  (if (>= (`self.HackingPoints`) HackingPointsToSpend)
    (set `self.HackingPoints` (`KismetMathLibrary.FClamp` (- (`self.HackingPoints`) (`local.HackingPointsToSpend`)) 0.0 100.0))
    (return true)
    (else
      (return false))))