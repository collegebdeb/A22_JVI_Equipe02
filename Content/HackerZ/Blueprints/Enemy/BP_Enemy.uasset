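; Patrolling enemy character that detects the player and can be hacked by spending the PocketHacker's hacking points.
; Detection events recolor its spotlight and switch walk/run speed; capsule contact with the player triggers detection.
; Hacking is delegated to AI_Controller_Enemy, while respawn resets transform, patrol index and sensor.
; DisplayHackingGUI tints dynamic materials by affordability and spikes a value that decays each tick, briefly revealing the camera-facing widget.
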(event `self.ReceiveTick`
  (params (DeltaSeconds :type "Float (single-precision)"))
  (bind _widget (`self.Widget`))
  (`self.UpdateMaterialHackDisplay`)
  (`SceneComponent.K2_SetWorldRotation` _widget (`KismetMathLibrary.FindLookAtRotation` (`SceneComponent.K2_GetComponentLocation` _widget) (`PlayerCameraManager.GetCameraLocation` (`GameplayStatics.GetPlayerCameraManager` 0))) false false))

(event `self.ReceiveBeginPlay`
  (bind _returnvalue (`AIBlueprintHelperLibrary.GetAIController` self))
  (`self.SetMaxWalkSpeed` (`self.WalkSpeed`))
  (`/Engine/EditorBlueprintResources/StandardMacros.IsValid` _returnvalue
    (:`Is Valid`
      (`self.K2_AttachToComponent` _returnvalue (`self.Mesh`) "Head" "KeepRelative" "KeepRelative" "KeepRelative" true)
      (set `self.SpawnTransform` (`SceneComponent.K2_GetComponentToWorld` (`self.CapsuleComponent`))))))

(event `OnDetectPlayer`
  (`LightComponent.SetLightColor` (`self.SpotLight`) (make `LinearColor` 1.0) true)
  (set `CharacterMovementComponent.MaxWalkSpeed` (`self.RunSpeed`) (`self.CharacterMovement`)))

(event `On Sense Player`
  (`LightComponent.SetLightColor` (`self.SpotLight`) (make `LinearColor` 1.0 1.0) true))

(event `OnLosePlayer`
  (`LightComponent.SetLightColor` (`self.SpotLight`) (make `LinearColor` 1.0 1.0 1.0) true)
  (set `CharacterMovementComponent.MaxWalkSpeed` (`self.WalkSpeed`) (`self.CharacterMovement`)))

(event `self.CapsuleComponent.OnComponentHit`
  (params (HitComponent :type "PrimitiveComponent Object Reference") (OtherActor :type "Actor Object Reference") (OtherComp :type "PrimitiveComponent Object Reference") (NormalImpulse :type "Vector Structure") (Hit :type "HitResult Structure (by ref)"))
  (cast `/Game/HackerZ/Blueprints/Player/FirstPersonBP/Blueprints/FirstPersonCharacter_Old` OtherActor)
  (bind _asai_controller_enemy (cast `/Game/HackerZ/Blueprints/Enemy/AI/AI_Controller_Enemy` (`AIBlueprintHelperLibrary.GetAIController` self)))
  (`/Game/HackerZ/Blueprints/Enemy/AI/AI_Controller_Enemy.OnDetectPlayer` _asai_controller_enemy))

(event `StartPatrolRoute`
  ;[1 1 1] Événement qui permet de débuter la route de patrouille
  (bind _asaicontroller (cast `AIController` (`self.GetController`)))
  (`BlackboardComponent.SetValueAsObject` (`AIBlueprintHelperLibrary.GetBlackboard` _asaicontroller) "PatrolRoute" (`self.PatrolRoute`)))

(fn `DisplayHackingGUI`
  (params (PocketHacker :type "/Game/HackerZ/Blueprints/Player/Components/BP_PocketHacker_SC Object Reference"))
  (`|ExecutionSequence`
    (:`then_0`
      (bind _enough_ (`/Game/HackerZ/Blueprints/Player/Components/BP_PocketHacker_SC.HasEnoughHackingPoints` (`local.PocketHacker`) (`self.HackingPointsRequiredToHack`)))
      (`MaterialInstanceDynamic.SetVectorParameterValue` (`self.Material2`) "DisplayHackingStatusColor" (`KismetMathLibrary.SelectColor` (struct :`R` 0.084637 :`G` 1.0 :`A` 1.0) (struct :`R` 1.0 :`A` 1.0) _enough_))
      (`MaterialInstanceDynamic.SetVectorParameterValue` (`self.Materials1`) "DisplayHackingStatusColor" (`KismetMathLibrary.SelectColor` (struct :`R` 0.084637 :`G` 1.0 :`A` 1.0) (struct :`R` 1.0 :`A` 1.0) _enough_))
      (set `self.MaterialHackDisplay` 2.0))))

(fn `GetHacked`
  (params (HackTime :type "Float (double-precision)") (PocketHacker :type "/Game/HackerZ/Blueprints/Player/Components/BP_PocketHacker_SC Object Reference"))
  (returns (Hacked :type "Actor Object Reference") (IsHacked :type Boolean))
  (bind _asai_controller_enemy (cast `/Game/HackerZ/Blueprints/Enemy/AI/AI_Controller_Enemy` (`AIBlueprintHelperLibrary.GetAIController` self)))
  (if (`/Game/HackerZ/Blueprints/Enemy/AI/AI_Controller_Enemy.IsHacked` _asai_controller_enemy)
    (return null false)
    (else
      (bind _isenoughpoints (`/Game/HackerZ/Blueprints/Player/Components/BP_PocketHacker_SC.SpendHackingPoints` PocketHacker (`self.HackingPointsRequiredToHack`)))
      (if _isenoughpoints
        (bind _asai_controller_enemy_2 (cast `/Game/HackerZ/Blueprints/Enemy/AI/AI_Controller_Enemy` (`AIBlueprintHelperLibrary.GetAIController` self)))
        (set `/Game/HackerZ/Blueprints/Enemy/AI/AI_Controller_Enemy.IsHacked` true _asai_controller_enemy_2)
        (`/Game/HackerZ/Blueprints/Enemy/AI/AI_Controller_Enemy.OnGetHacked` _asai_controller_enemy_2 (`local.HackTime`))
        (`KismetSystemLibrary.PrintString` "Got Hacked!")
        (`GameplayStatics.PlaySoundAtLocation` "/Game/HackerZ/Blueprints/Enemy/Audio/Glitch_sound.Glitch_sound" (`self.K2_GetActorLocation` self) (struct) 0.5 1.0 0.0 null null null null)
        (return self true)
        (else
          (`KismetSystemLibrary.PrintString` "Not enough hacking points to hack" true false (struct :`R` 1.0 :`G` 0.03671 :`A` 1.0))
          (return null false))))))

(fn `Respawn`
  (bind _patrolroute (`self.PatrolRoute`))
  (`self.K2_SetActorTransform` (`self.SpawnTransform`) false true)
  (`/Engine/EditorBlueprintResources/StandardMacros.IsValid` _patrolroute
    (:`Is Valid`
      (set `/Game/HackerZ/Blueprints/Enemy/BP_PatrolRoute.CurrentPatrolPointIndex` (`/Game/HackerZ/Blueprints/Enemy/BP_PatrolRoute.FirstPatrolPointIndex` _patrolroute) _patrolroute))
    (:`Is Not Valid`
      _))
  (bind _asai_controller_enemy (cast `/Game/HackerZ/Blueprints/Enemy/AI/AI_Controller_Enemy` (`AIBlueprintHelperLibrary.GetAIController` self)))
  (set `/Game/HackerZ/Blueprints/Enemy/AI/AI_Controller_Enemy.Sensor` 0.0 _asai_controller_enemy))

(fn `ReturnHackingPointsRequired`
  (returns (HackingPointsRequired :type "Float (double-precision)"))
  (return 0.0))

(fn `SetMaxWalkSpeed`
  (params (MaxWalkSpeed :type "Float (double-precision)"))
  (set `CharacterMovementComponent.MaxWalkSpeed` MaxWalkSpeed (`self.CharacterMovement`)))

(fn `UpdateMaterialHackDisplay`
  (bind _widget (`self.Widget`))
  (bind _output_get (set `self.MaterialHackDisplay` (`KismetMathLibrary.FInterpTo` (`self.MaterialHackDisplay`) 0.0 (`GameplayStatics.GetWorldDeltaSeconds`) 3.0)))
  (`MaterialInstanceDynamic.SetScalarParameterValue` (`self.Material2`) "DisplayHack" _output_get)
  (`MaterialInstanceDynamic.SetScalarParameterValue` (`self.Materials1`) "DisplayHack" _output_get)
  (if (>= (`self.MaterialHackDisplay`) 1.0)
    (`SceneComponent.SetHiddenInGame` _widget false false)
    (else
      (`SceneComponent.SetHiddenInGame` _widget true false))))

(fn `UserConstructionScript`
  (bind _mesh (`self.Mesh`))
  (bind _returnvalue (`PrimitiveComponent.CreateDynamicMaterialInstance` _mesh 0 "/Game/HackerZ/Characters/Mannequins/Materials/Instances/Manny/MI_Manny_02.MI_Manny_02" "None"))
  (set `self.Material2` _returnvalue)
  (bind _returnvalue_2 (`PrimitiveComponent.CreateDynamicMaterialInstance` _mesh 1 "/Game/HackerZ/Characters/Mannequins/Materials/Instances/Manny/MI_Manny_01.MI_Manny_01" "None"))
  (set `self.Materials1` _returnvalue_2))